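; BP_AutoAttack is a skill that performs an auto-attack, dealing base melee damage to its defenders.
; On execution it gathers defenders, casts each to BrendenmoorCharacter and applies truncated damage through StandardAttributes.
; Health is checked before and after each hit, and a dead enemy or empty defender list stops auto-attack through the attacker's BattleSystemComponent.
; Debug strings print when no defenders are found and when the attack stops.
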(event EventExecuteSkill
  (bind _defenders (Variables|Default|GetDefenders))
  (bind _returnvalue (Utilities|Array|Length _defenders))
  (CallFunction|GetDefenders)
  (if (> _returnvalue 0)
    (for _array_element _defenders
      (bind _asbrendenmoor_character (Utilities|Casting|CastToBrendenmoorCharacter _array_element))
      (bind _isdead (CallFunction|CheckifEnemyIsDead _asbrendenmoor_character))
      (if _isdead
        (CallFunction|StopAutoAttack)
        (else
          (Class|CStandardAttributes|TakeDamage (Variables|/Script/Brendenmoor.BrendenmoorCharacter|GetstandardAttributes _asbrendenmoor_character) (Math|Float|Truncate (Class|CBaseSkill|CalculateBaseMeleeDamage)))
          (bind _isdead_2 (CallFunction|CheckifEnemyIsDead _asbrendenmoor_character))
          (if _isdead_2
            (CallFunction|StopAutoAttack)))))
    (else
      (Development|PrintString (Utilities|String|ToString(Integer) _returnvalue) true true "(R=1.000000,G=0.233938,B=0.000000,A=1.000000)")
      (CallFunction|StopAutoAttack))))

(fn ConstructionScript
  (|CallParentFunction))

(fn StopAutoAttack
  (bind _asbrendenmoor_character (Utilities|Casting|CastToBrendenmoorCharacter (Variables|Default|GetAttacker)))
  (Class|BattleSystemComponent|StopAutoAttack (Variables|/Script/Brendenmoor.BrendenmoorCharacter|GetbattleSystemComponent _asbrendenmoor_character))
  (Development|PrintString "stop auto attack"))

(fn CheckifEnemyIsDead
  (params (Enemy :type Brendenmoor%20Character%20Object%20Reference))
  (return (<= (Variables|/Script/Brendenmoor.CStandardAttributes|GetCurrentHealth (Variables|/Script/Brendenmoor.BrendenmoorCharacter|GetstandardAttributes Enemy)) 0)))