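; Auto-attack skill Blueprint that deals base melee damage from an attacker to its defenders.
; ExecuteSkill casts the Attacker to BrendenmoorCharacter, then loops over Defenders, applying truncated CalculateBaseMeleeDamage through each one's StandardAttributes.TakeDamage.
; Debug prints show the skill, attacker name and damage, with the damage calculation called again for the printout.
; The parent ExecuteSkill call is never run.
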(event EventBeginPlay)

(event Collision|EventActorBeginOverlap
  (params (OtherActor :type Actor%20Object%20Reference)))

(event EventTick
  (params (DeltaSeconds :type Float%20%28single-precision%29)))

(event EventExecuteSkill
  (bind _returnvalue (Class|CBaseSkill|CalculateBaseMeleeDamage))
  (bind _returnvalue_2 (Math|Float|Truncate _returnvalue))
  (Development|PrintText "Auto Attack" true true "(R=0.193527,G=0.023669,B=0.235000,A=1.000000)" 5.0)
  (bind _asbrendenmoor_character (Utilities|Casting|CastToBrendenmoorCharacter (Variables|Default|GetAttacker)))
  (Development|PrintString (Utilities|String|ToString(Name) (Variables|/Script/Brendenmoor.BrendenmoorCharacter|GetCharacterName _asbrendenmoor_character)))
  (for _array_element (Variables|Default|GetDefenders)
    (bind _asbrendenmoor_character_2 (Utilities|Casting|CastToBrendenmoorCharacter _array_element))
    (Class|CStandardAttributes|TakeDamage (Variables|/Script/Brendenmoor.BrendenmoorCharacter|GetstandardAttributes _asbrendenmoor_character_2) _returnvalue_2)
    (Development|PrintString (Utilities|String|ToString(Integer) _returnvalue_2) true true "(R=0.061279,G=1.000000,B=0.000000,A=1.000000)")))

(fn ConstructionScript)