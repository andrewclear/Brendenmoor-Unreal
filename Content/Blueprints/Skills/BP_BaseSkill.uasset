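; BP_BaseSkill is a base skill Blueprint that selects the defenders a skill affects.
; GetDefenders switches on TargetTypeEnum to one function each for single target, AOE around target, AOE around attacker and AOE in front.
; Only the in-front function is implemented: it adds the nearest enemy from the TargettingSystemComponent on the Attacker's owner to Defenders, with no area or facing check.
; The other targeting functions and all events are empty.
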(event EventBeginPlay)

(event Collision|EventActorBeginOverlap
  (params (OtherActor :type Actor%20Object%20Reference)))

(event EventTick
  (params (DeltaSeconds :type Float%20%28single-precision%29)))

(fn ConstructionScript)

(fn GetDefenderSingleTarget)

(fn GetDefendersAOETarget)

(fn GetDefendersAOEAttacker)

(fn GetDefendersAOEAttackerinFront
  (bind _returnvalue (Class|TargettingSystemComponent|GetNearestEnemy (Actor|GetComponentbyClass (Components|GetOwner (Variables|Default|GetAttacker)) "/Script/Brendenmoor.TargettingSystemComponent")))
  (Utilities|Array|Add (Variables|Default|GetDefenders) _returnvalue))

(fn GetDefenders
  (switch Utilities|FlowControl|Switch|SwitchonETargetType (Variables|Default|GetTargetTypeEnum)
    (:VE_Single
      (CallFunction|GetDefenderSingleTarget))
    (:VE_AOEAroundTarget
      (CallFunction|GetDefendersAOETarget))
    (:VE_AOEAroundAttacker
      (CallFunction|GetDefendersAOEAttacker))
    (:VE_AOEInFrontOfAttacker
      (CallFunction|GetDefendersAOEAttackerinFront))))