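; BP_Attributes is a component that derives a character's combat stats from primary attributes.
; UpdateAttributes computes physical and magic defense plus melee, magic and ranged attack as weighted sums of Strength, Vitality, Agility and Inteligence.
; Getter functions expose these cached results and a separate BaseAttackSpeed, which the update leaves untouched.
; Nothing runs on BeginPlay or Tick, and the component does not call UpdateAttributes itself.
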(event EventBeginPlay)

(event EventTick
  (params (DeltaSeconds :type Float%20%28single-precision%29)))

(fn UpdateAttributes
  (bind _strength (Variables|BaseAttributes|GetStrength))
  (bind _inteligence (Variables|BaseAttributes|GetInteligence))
  ;[0 0 0] Calculate Defense
  ;;[1 0 0] Calculate Physical Defense
  (Variables|CalculateAttributes|SetPhysicalDefense (+ (Variables|BaseAttributes|GetStrength) (* (Variables|BaseAttributes|GetVitality) 2)))
  ;;[0 0.06613 1] Calculate Magic Defense
  (Variables|CalculateAttributes|SetMagicDefense (+ (* (Variables|BaseAttributes|GetVitality) 2) (Variables|BaseAttributes|GetInteligence)))
  ;[0 0 0] Calculate Attack
  ;;[0 0.01 1] Calculate Magic Attack
  (Variables|CalculateAttributes|SetMagicAttack (+ _inteligence (* _inteligence 2)))
  ;;[1 0 0] Calculate Melee Attack
  (Variables|CalculateAttributes|SetMeleeAttack (+ _strength (* _strength 2)))
  ;;[1 0 0] Calculate Ranged Attack
  (Variables|CalculateAttributes|SetRangedAttack (+ (Variables|BaseAttributes|GetStrength) (* (Variables|BaseAttributes|GetAgility) 2))))

(fn GetPhysicalDefense
  (return (Variables|CalculateAttributes|GetPhysicalDefense)))

(fn GetMagicDefense
  (return (Variables|CalculateAttributes|GetMagicDefense)))

(fn GetMeleeAttack
  (return (Variables|CalculateAttributes|GetMeleeAttack)))

(fn GetMagicAttack
  (return (Variables|CalculateAttributes|GetMagicAttack)))

(fn GetRangedAttack
  (return (Variables|CalculateAttributes|GetRangedAttack)))

(fn GetBaseAttackSpeed
  (return (Variables|CalculateAttributes|GetBaseAttackSpeed)))