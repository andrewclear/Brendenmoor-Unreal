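; Targeting system component that collects pawns near its owning actor, apparently early work in progress.
; The GetAllNearbyActors event runs a multi-sphere object trace for Pawns at the owner's location, using a configurable radius.
; Each hit actor is added uniquely to ArrayAllLoadedCharacters, with no removal and no class filter, as the BrendenmoorCharacter cast is disconnected.
; Nothing here calls the event, and Test is only a debug print.
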(event EventBeginPlay)

(event EventTick
  (params (DeltaSeconds :type Float%20%28single-precision%29)))

(event EventGetAllNearbyActors
  (bind _returnvalue (Components|GetOwner))
  (bind _returnvalue_2 (Transformation|GetActorTransform _returnvalue))
  (bind _location (Math|Transform|BreakTransform _returnvalue_2))
  (bind (_outhits _returnvalue_3) (Collision|MultiSphereTraceForObjects _location _location (Variables|Default|GetRadiusForSphereTrace) (Utilities|Array|MakeArray "ObjectTypeQuery3") false 0 "None"))
  (if _returnvalue_3
    (for _array_element _outhits
      (Utilities|Array|AddUnique (Variables|Default|GetarrayAllLoadedCharacters) (.HitActor (Collision|BreakHitResult _array_element))))))

(fn Test
  (Development|PrintString "Hello"))