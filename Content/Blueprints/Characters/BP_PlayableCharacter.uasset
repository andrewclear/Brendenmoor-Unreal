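; Playable character Blueprint that currently serves as a debug readout for enemy targeting.
; Each Tick it asks its TargettingSystemComponent for the nearest enemy and casts the result to BrendenmoorCharacter.
; It prints that character's name and the component's debug distance on screen, or a failure message if the cast fails.
; Player possession by character name and a loop over all loaded characters are left unconnected, so neither runs.
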(event EventBeginPlay)

(event Collision|EventActorBeginOverlap
  (params (OtherActor :type Actor%20Object%20Reference)))

(event EventTick
  (params (DeltaSeconds :type Float%20%28single-precision%29))
  (bind _returnvalue (Actor|GetComponentbyClass "/Script/Brendenmoor.TargettingSystemComponent"))
  (bind _returnvalue_2 (Class|TargettingSystemComponent|GetNearestEnemy _returnvalue))
  (bind _asbrendenmoor_character (Utilities|Casting|CastToBrendenmoorCharacter _returnvalue_2)
    (:then
      (Development|PrintString (Utilities|String|ToString(Name) (Variables|/Script/Brendenmoor.BrendenmoorCharacter|GetCharacterName _asbrendenmoor_character)) true true "(R=0.523285,G=0.000000,B=0.680000,A=1.000000)")
      (Development|PrintString (Utilities|String|ToString(Float) (Variables|/Script/Brendenmoor.TargettingSystemComponent|GetDebugDistance _returnvalue)) true true "(R=1.000000,G=0.855670,B=0.000000,A=1.000000)"))
    (:CastFailed
      (Development|PrintString "Cast Failed" true true "(R=1.000000,G=0.042102,B=0.000000,A=1.000000)"))))

(fn ConstructionScript)