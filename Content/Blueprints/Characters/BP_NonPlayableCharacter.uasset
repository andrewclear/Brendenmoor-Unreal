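; Non-playable character Blueprint that removes itself on death and polls for nearby enemies.
; Each Tick destroys the actor once StandardAttributes current health reaches zero or below, otherwise asks its TargettingSystemComponent for the nearest enemy.
; The enemy result drives no behavior: a debug chain that casts it to BrendenmoorCharacter and prints its name is left disconnected.
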(event EventBeginPlay)

(event Collision|EventActorBeginOverlap
  (params (OtherActor :type Actor%20Object%20Reference)))

(event EventTick
  (params (DeltaSeconds :type Float%20%28single-precision%29))
  (if (<= (Variables|/Script/Brendenmoor.CStandardAttributes|GetCurrentHealth (Variables|Default|GetstandardAttributes)) 0)
    (Actor|DestroyActor)
    (else
      (bind _returnvalue (Class|TargettingSystemComponent|GetNearestEnemy (Actor|GetComponentbyClass "/Script/Brendenmoor.TargettingSystemComponent"))))))

(fn ConstructionScript)