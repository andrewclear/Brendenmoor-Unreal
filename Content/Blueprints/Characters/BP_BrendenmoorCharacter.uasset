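; BP_BrendenmoorCharacter is a character Blueprint that builds a list of the other BrendenmoorCharacter actors in the scene.
; On BeginPlay, GetAllCharactersInScene finds all actors of that class, skips itself and adds each one uniquely to ArrayAllCharacters.
; It prints each found character's name on screen, then passes the finished array to UpdateCharacterArray.
; The list is gathered only at BeginPlay, as Tick and overlap events are unused.
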(event EventBeginPlay
  (CallFunction|GetAllCharactersinScene))

(event Collision|EventActorBeginOverlap
  (params (OtherActor :type Actor%20Object%20Reference)))

(event EventTick
  (params (DeltaSeconds :type Float%20%28single-precision%29)))

(fn ConstructionScript)

(fn GetAllCharactersinScene
  (bind _outactors (Actor|GetAllActorsOfClass "/Script/Brendenmoor.BrendenmoorCharacter"))
  (for _array_element _outactors
    (if (not (== _array_element self))
      (Utilities|Array|AddUnique (LocalVariables|GetarrayAllCharacters) _array_element)
      (Development|PrintString (Utilities|String|ToString(Name) (Variables|/Script/Brendenmoor.BrendenmoorCharacter|GetCharacterName _array_element)) true true "(R=1.000000,G=0.067083,B=0.166763,A=1.000000)")))
  (Class|BrendenmoorCharacter|UpdateCharacterArray (LocalVariables|GetarrayAllCharacters)))