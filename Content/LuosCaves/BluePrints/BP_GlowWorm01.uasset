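; BP_GlowWorm01 is a glow worm decal actor in the LuosCaves content, with a configurable emissive look.
; Its construction script creates a dynamic material instance on the Decal1 component.
; It then copies the Blueprint's four color variables, tiling and emissive power into that material's parameters.
; The script holds no runtime logic, only this construction-time setup.
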(fn ConstructionScript
  (bind _decal1 (Variables|Default|GetDecal1))
  (bind _returnvalue (Rendering|Material|CreateDynamicMaterialInstance _decal1 :!class /Script/Engine.DecalComponent))
  (Rendering|Components|Decal|SetDecalMaterial _decal1 _returnvalue)
  (Rendering|Material|SetVectorParameterValue _returnvalue "Color1" (Variables|Default|GetColor1) :!class /Script/Engine.MaterialInstanceDynamic)
  (Rendering|Material|SetVectorParameterValue _returnvalue "Color2" (Variables|Default|GetColor2) :!class /Script/Engine.MaterialInstanceDynamic)
  (Rendering|Material|SetVectorParameterValue _returnvalue "Color3" (Variables|Default|GetColor3) :!class /Script/Engine.MaterialInstanceDynamic)
  (Rendering|Material|SetVectorParameterValue _returnvalue "Color4" (Variables|Default|GetColor4) :!class /Script/Engine.MaterialInstanceDynamic)
  (Rendering|Material|SetScalarParameterValue _returnvalue "Tiling" (Variables|Default|GetTiling) :!class /Script/Engine.MaterialInstanceDynamic)
  (Rendering|Material|SetScalarParameterValue _returnvalue "emissivePower" (Variables|Default|GetEmissive) :!class /Script/Engine.MaterialInstanceDynamic))