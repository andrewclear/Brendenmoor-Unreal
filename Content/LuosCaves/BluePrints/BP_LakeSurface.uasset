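; Cave lake surface actor that shows rippling water with a repeating drip sound at the ripple origin.
; The construction script scales the mesh, passes origin, time offset and fadeout radius to a dynamic MI_LakeWater material, then reads back speed and period.
; At BeginPlay, a looping timer starts after the time offset and plays drips at intervals derived from the material's speed, tying audio timing to the ripple parameters.
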(event Custom|Play%20Drip%20Sound
  (Audio|PlaySoundatLocation "/Game/LuosCaves/Sounds/S_Drips_Wet_Regular_cue.S_Drips_Wet_Regular_cue" (Math|Transform|TransformLocation (Transformation|GetActorTransform) (Variables|Default|GetRipple%20Origin)) 1e+01))

(event EventBeginPlay
  (Utilities|FlowControl|Delay (Variables|Default|GetTimeOffset))
  (Utilities|Time|SetTimerbyEvent (delegate Custom|Play%20Drip%20Sound) (/ 1.0 (Variables|Default|GetDripSpeed)) true))

(fn ConstructionScript
  (bind _lakesurfacemesh (Variables|Default|GetLakeSurfaceMesh))
  (bind _lakesurfacescale (Variables|Default|GetLakeSurfaceScale))
  (bind _returnvalue (Rendering|Material|CreateDynamicMaterialInstance _lakesurfacemesh 0 "/Game/LuosCaves/Materials/Extra_Prop_Instances/MI_LakeWater.MI_LakeWater" :!class /Script/Engine.PrimitiveComponent))
  (Rendering|Material|SetMaterial _lakesurfacemesh 0 _returnvalue)
  (Rendering|Material|SetVectorParameterValue _returnvalue "RipplesOrigin" (Math|Conversions|ToLinearColor(Vector) (Math|Transform|TransformLocation (Transformation|GetActorTransform) (Variables|Default|GetRipple%20Origin))) :!class /Script/Engine.MaterialInstanceDynamic)
  (Rendering|Material|SetScalarParameterValue _returnvalue "TimeOffset" (Variables|Default|GetTimeOffset) :!class /Script/Engine.MaterialInstanceDynamic)
  (Rendering|Material|SetScalarParameterValue _returnvalue "Fadeout Radius" (Variables|Default|GetFadeoutRadius) :!class /Script/Engine.MaterialInstanceDynamic)
  (Transformation|SetRelativeScale3D (Variables|Default|GetLakeSurfaceMesh) (Math|Vector|MakeVector (.x _lakesurfacescale) (.y _lakesurfacescale) 1.0))
  (bind _returnvalue_2 (Rendering|Material|GetScalarParameterValue _returnvalue "Speed" :!class /Script/Engine.MaterialInstanceDynamic))
  (Variables|Default|SetDripSpeed _returnvalue_2)
  (bind _returnvalue_3 (Rendering|Material|GetScalarParameterValue _returnvalue "RipplePeriod" :!class /Script/Engine.MaterialInstanceDynamic))
  (Variables|Default|SetPeriod _returnvalue_3))