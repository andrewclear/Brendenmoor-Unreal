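; Fantasy lamp prop Blueprint for the Luos Caves content, configurable by color, emissive power and light falloff.
; The construction script gives the lamp mesh a dynamic orange-lamp material instance driven by the color and emissive settings.
; It layers three co-located point lights in that color for close, medium and far range.
; The medium light derives from geometric means of the close and far radius and brightness, with its brightness further reduced.
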(fn ConstructionScript
  (bind _returnvalue (Math|Transform|MakeTransform "82.000000,-20.000000,110.000000"))
  (bind _sm_lprop_lamp_3_0 (Variables|Default|GetSM_LProp_Lamp_3_0))
  ;[1 1 1] Material
  (bind _returnvalue_2 (Rendering|Material|CreateDynamicMaterialInstance _sm_lprop_lamp_3_0 0 "/Game/LuosCaves/Materials/Extra_Prop_Instances/MI_Prop_Lamp_Orange.MI_Prop_Lamp_Orange" :!class /Script/Engine.PrimitiveComponent))
  (Variables|Default|SetDynMaterial _returnvalue_2)
  (Rendering|Material|SetMaterial _sm_lprop_lamp_3_0 0 (Variables|Default|GetDynMaterial))
  (Rendering|Material|SetScalarParameterValue (Variables|Default|GetDynMaterial) "2. Lamp Emissive Power" (Variables|Default|GetEmissivePower) :!class /Script/Engine.MaterialInstanceDynamic)
  (Rendering|Material|SetVectorParameterValue (Variables|Default|GetDynMaterial) "1. Lamp Color" (Variables|Default|GetColor) :!class /Script/Engine.MaterialInstanceDynamic)
  (Variables|LightRange|SetLightRadMed (Math|Float|Sqrt (* (Variables|LightRange|GetLightRadClose) (Variables|LightRange|GetLightRadfar))))
  (Variables|Default|SetLightBrightnessMed (/ (Math|Float|Sqrt (* (Variables|Default|GetLightBrightnessClose) (Variables|Default|GetLightBrightnessFar))) 1.5))
  ;[1 1 1] LightClose
  (bind _returnvalue_3 (AddComponent|AddPointLightComponent false _returnvalue))
  (Rendering|Components|Light|SetIntensity _returnvalue_3 (Variables|Default|GetLightBrightnessClose))
  (Rendering|Lighting|SetAttenuationRadius _returnvalue_3 (Variables|LightRange|GetLightRadClose))
  (Rendering|Components|Light|SetLightColor _returnvalue_3 (Variables|Default|GetColor))
  ;[1 1 1] LightMedium
  (bind _returnvalue_4 (AddComponent|AddPointLightComponent false _returnvalue))
  (Rendering|Components|Light|SetIntensity _returnvalue_4 (Variables|Default|GetLightBrightnessMed))
  (Rendering|Lighting|SetAttenuationRadius _returnvalue_4 (Variables|LightRange|GetLightRadMed))
  (Rendering|Components|Light|SetLightColor _returnvalue_4 (Variables|Default|GetColor))
  ;[1 1 1] LightFar
  (bind _returnvalue_5 (AddComponent|AddPointLightComponent false _returnvalue))
  (Rendering|Components|Light|SetIntensity _returnvalue_5 (Variables|Default|GetLightBrightnessFar))
  (Rendering|Lighting|SetAttenuationRadius _returnvalue_5 (Variables|LightRange|GetLightRadfar))
  (Rendering|Components|Light|SetLightColor _returnvalue_5 (Variables|Default|GetColor)))